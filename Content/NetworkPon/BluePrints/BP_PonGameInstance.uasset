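; Game instance for NetworkPon that hosts and joins two-connection LAN sessions.
; CreateSession creates the session, then opens the Game level as a listen server.
; JoinSession searches LAN for a single session and joins the first result.
; Network and travel failures, like each session step, are only printed to screen, with no recovery handling.
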(event Custom|CreateSession
  (|Session (Game|GetPlayerController 0) 2 true
    (:OnSuccess
      (Development|PrintString "Success Create Session")
      (Game|OpenLevel(byName) "Game" true "listen"))
    (:OnFailure
      (Development|PrintString "Fail Create Session"))))

(event Custom|JoinSession
  (bind _results (|FindSessions (Game|GetPlayerController 0) 1 true)
    (:OnSuccess
      (Development|PrintString "Success Find Session")
      (|JoinSession (Game|GetPlayerController 0) (Utilities|Array|Get(acopy) _results)
        (:OnSuccess
          (Development|PrintString "Success Join Session"))
        (:OnFailure
          (Development|PrintString "Fail Join Session"))))
    (:OnFailure
      (Development|PrintString "Fail Find Session"))))

(event EventHandleNetworkError
  (params (FailureType :type ENetworkFailure%20Enum :default "NetDriverAlreadyExists") (bIsServer :type Boolean))
  (switch Utilities|FlowControl|Switch|SwitchonENetworkFailure FailureType
    (:NetDriverAlreadyExists
      _)
    (:NetDriverCreateFailure
      _)
    (:NetDriverListenFailure
      _)
    (:ConnectionLost
      _)
    (:ConnectionTimeout
      _)
    (:FailureReceived
      _)
    (:OutdatedClient
      _)
    (:OutdatedServer
      _)
    (:PendingConnectionFailure
      _)
    (:NetGuidMismatch
      _)
    (:NetChecksumMismatch
      _))
  (Development|PrintString (Utilities|String|EnumtoString FailureType) true true "(R=0.000000,G=0.660000,B=1.000000,A=1.000000)" 1e+02))

(event EventHandleTravelError
  (params (FailureType :type ETravelFailure%20Enum :default "NoLevel"))
  (switch Utilities|FlowControl|Switch|SwitchonETravelFailure FailureType
    (:NoLevel
      _)
    (:LoadMapFailure
      _)
    (:InvalidURL
      _)
    (:PackageMissing
      _)
    (:PackageVersion
      _)
    (:NoDownload
      _)
    (:TravelFailure
      _)
    (:CheatCommands
      _)
    (:PendingNetGameCreateFailure
      _)
    (:CloudSaveFailure
      _)
    (:ServerTravelFailure
      _)
    (:ClientTravelFailure
      _))
  (Development|PrintString (Utilities|String|EnumtoString FailureType)))