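; BP_PlayerFacade links a player to a target goal and a HUD, keeping that player's score.
; ConnectPlayer stores the player and binds OnGoalEvent to the opponent's goal, which adds a point when the ball enters.
; Each goal passes the new score to UpdateScoreHud, commented as server-only, which forwards it to PlayerHud.
; Score has a RepNotify that only prints a debug message.
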(event Custom|UpdateScoreHud
  (params (Score :type Integer))
  ;[1 1 1] サーバーにだけスコアを伝える
  (Default|UpdateScoreHud (Variables|Default|GetPlayerHud) Score))

(event Custom|ConnectPlayer
  (params (Player :type BP%20Bar%20Object%20Reference))
  ;[1 1 1] 相手ゴールに球が入ったときに得点を入れる。
  (Variables|Default|SetPlayer Player)
  (EventDispatchers|AssignOnGoal (Variables|Default|GetTargetGoal) (delegate Custom|OnGoalEvent)))

(event Custom|OnGoalEvent
  ;[1 1 1] 相手ゴールに球が入ったときに得点を入れる。
  (bind _output_get (Variables|Default|SetScore (+ (Variables|Default|GetScore) 1)))
  (CallFunction|UpdateScoreHud _output_get))

(fn ConstructionScript)

(fn OnRepScore
  (Development|PrintString "Change!!" true true "(R=0.000000,G=0.660000,B=1.000000,A=1.000000)" 1e+02))