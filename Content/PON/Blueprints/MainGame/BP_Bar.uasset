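; BP_Bar is an input-driven bar actor, apparently a paddle, that moves along the world Y axis in the PON main game.
; The MoveUp axis feeds UpdateMovement, which stores a per-frame Velocity scaled by Speed and world delta time, zeroed when there is no input.
; Tick calls Movement, which applies that offset with a sweep so blocking collisions stop the bar.
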(event Custom|UpdateMovement
  (params (AxisValue :type Float%20%28single-precision%29))
  (bind _returnvalue (Utilities|Time|GetWorldDeltaSeconds))
  (bind _speed (Variables|Default|GetSpeed))
  (bind _returnvalue_2 (* _speed _returnvalue))
  (bind _returnvalue_3 (* AxisValue _returnvalue_2))
  (if (> (Math|Float|Absolute(Float) _returnvalue_3) 0.0)
    (Variables|Default|SetVelocity (Math|Vector|MakeVector 0.0 _returnvalue_3 0.0))
    (else
      (Variables|Default|SetVelocity "0, 0, 0"))))

(event Custom|Movement
  (Transformation|AddActorWorldOffset (Variables|Default|GetVelocity) true))

(event EventTick
  (params (DeltaSeconds :type Float%20%28single-precision%29))
  (CallFunction|Movement))

(event Input|AxisEvents|InputAxisMoveUp
  (params (AxisValue :type Float%20%28single-precision%29))
  (CallFunction|UpdateMovement AxisValue))

(fn ConstructionScript)