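; Game mode for two-player Pong that seats players and keeps a ball in play.
; On player restart, it moves the bar to a tagged PlayerStart (local controller "2", otherwise "1") and links it to the matching BP_PlayerFacade.
; After a delay it switches the view to the GameCamera, and two registered bars fire OnEndPlayerLogin to start the game.
; Balls spawn at BallSpawnLoc target points and respawn through their OnKill event.
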(event Custom|KillEvent
  ;[1 1 1] ボールを生み出す
  (CallFunction|SpawnBall))

(event Custom|SpawnBall
  ;[1 1 1] ボールを生み出す
  (bind _outactors (Actor|GetAllActorsOfClass "/Script/Engine.TargetPoint"))
  (for _array_element _outactors
    (if (Actor|ActorHasTag _array_element "BallSpawnLoc")
      (bind _returnvalue (Game|SpawnActorfromClass "/Game/PON/Blueprints/MainGame/BP_Ball.BP_Ball_C" (Math|Transform|MakeTransform (Transformation|GetActorLocation _array_element) "0, 0, 0" "0.500000,0.500000,0.500000") "Undefined" 0 0))
      (Default|Init _returnvalue)
      (EventDispatchers|AssignOnKill _returnvalue (delegate Custom|KillEvent)))))

(event Custom|StartGame
  ;[1 1 1] ゲーム開始
  (CallFunction|SpawnBall))

(event EventBeginPlay
  ;[1 1 1] GameCtrlに制御のもろもろを任せる。
  (EventDispatchers|BindEventtoOnEndPlayerLogin (delegate Custom|StartGame)))

(event EventOnRestartPlayer
  (params (NewPlayer :type Controller%20Object%20Reference))
  ;[1 1 1] StartPlayerの生成
  (bind _asplayer_controller (Utilities|Casting|CastToPlayerController NewPlayer))
  (bind _output_get (Variables|Default|SetPlayerCtrl _asplayer_controller))
  ;;[1 1 1] 各プレイヤー定位置に出現させる
  (bind _asbp_bar (Utilities|Casting|CastToBP_Bar (Pawn|GetControlledPawn (Variables|Default|GetPlayerCtrl))))
  (Transformation|SetActorTransform _asbp_bar (CallFunction|GetPlayerStartTrans (select (Pawn|IsLocalPlayerController _output_get) "2" "1")))
  (Utilities|Array|Add (Variables|Default|GetPlayers) _asbp_bar)
  ;;[1 1 1] ゴールとの紐づけを行う
  (bind _outactors (Actor|GetAllActorsOfClass "/Game/PON/Blueprints/MainGame/BP_PlayerFacade.BP_PlayerFacade_C"))
  (for _array_element _outactors
    (if (Actor|ActorHasTag _array_element (Utilities|String|StringToName (Utilities|String|BuildString(Name) "Player" "" (select (Pawn|IsLocalPlayerController _output_get) "2" "1") "")))
      (Default|ConnectPlayer _array_element _asbp_bar)
      ;;[1 1 1] カメラを見下ろしに設定
      (Utilities|FlowControl|Delay 1.0)
      (bind _outactors_2 (Actor|GetAllActorsOfClass "/Script/Engine.CameraActor"))
      (for _array_element_2 _outactors_2
        (if (Actor|ActorHasTag _array_element_2 "GameCamera")
          (Game|Player|SetViewTargetwithBlend (Variables|Default|GetPlayerCtrl) _array_element_2 0.0 "VTBlend_Linear" 0.0 false)
          ;;[1 1 1] プレイヤーがそろった時点で開始
          (if (== (Utilities|Array|Length (Variables|Default|GetPlayers)) 2)
            (Default|CallOnEndPlayerLogin)))))))

(fn ConstructionScript)

(fn GetCurrentJoinPlayerNum
  (bind _outactors (Actor|GetAllActorsOfClass "/Script/Engine.PlayerController"))
  (return (Utilities|Array|Length _outactors)))

(fn GetGameCamera
  (bind _outactors (Actor|GetAllActorsOfClass 0))
  (return (Utilities|Array|Get(acopy) _outactors)))

(fn GetSpawnTrans
  (params (SpawnPointName :type Name))
  (bind _outactors (Actor|GetAllActorsOfClass "/Script/Engine.PlayerStart"))
  (for _array_element _outactors
    (if (Utilities|Name|Equal(Name) (Variables|/Script/Engine.PlayerStart|GetPlayerStartTag _array_element) SpawnPointName)
      (return (Transformation|GetActorTransform _array_element)))))

(fn AddPlayer
  (params (NewItem :type BP%20Bar%20Object%20Reference%20%28by%20ref%29))
  (bind _players (Variables|Default|GetPlayers))
  (bind _returnvalue (Utilities|Array|Add _players NewItem))
  (if (== (Utilities|Array|Length _players) 2)
    (Default|CallOnEndPlayerLogin))
  (return _returnvalue))

(fn GetBarNum
  (return (Utilities|Array|Length (Variables|Default|GetPlayers))))

(fn GetPlayerStartTrans
  (params (PlayerIndex :type Name))
  (bind _outactors (Actor|GetAllActorsOfClass "/Script/Engine.PlayerStart"))
  (for _array_element _outactors
    (if (Utilities|Name|Equal(Name) (Variables|/Script/Engine.PlayerStart|GetPlayerStartTag _array_element) PlayerIndex)
      (return (Transformation|GetActorTransform _array_element))))
  (return (Transformation|GetActorTransform _array_element)))