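; BP_Ball is the bouncing ball actor for the PON game, moved by a swept world offset every tick.
; Init, intended for server-only calls and thus not replicated, launches it forward with a slight rightward bias.
; BallMesh hits reflect the velocity off the surface normal and play spark and sound effects.
; Kill fires OnKill, plays an explosion, hides the ball, disables collision and sets a delayed lifespan for cleanup.
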(event OnComponentHit(BallMesh)
  (params (HitComponent :type Primitive%20Component%20Object%20Reference) (OtherActor :type Actor%20Object%20Reference) (OtherComp :type Primitive%20Component%20Object%20Reference) (NormalImpulse :type Vector :default "0, 0, 0") (Hit :type Hit%20Result%20Structure%20%28by%20ref%29))
  (CallFunction|RefrectBall Hit OtherActor))

(event Custom|RefrectBall
  (params (Hit :type Hit%20Result%20Structure) (OtherActor :type Actor%20Object%20Reference))
  (Variables|Default|SetVelocity (Math|Vector|GetReflectionVector (Variables|Default|GetVelocity) (.Normal (Collision|BreakHitResult Hit))))
  (CallFunction|PlayEffect))

(event Custom|Move
  (Transformation|AddActorWorldOffset (* (Variables|Default|GetVelocity) (* (Variables|Default|GetMoveSpeed) (Utilities|Time|GetWorldDeltaSeconds))) true))

(event Custom|Init
  ;[1 1 1] サーバ側で呼び出されることが決まっているので関数レプリケートを行っていない
  (Variables|Default|SetVelocity (+ (Transformation|GetActorForwardVector) (* (Transformation|GetActorRightVector) 0.2))))

(event Custom|Kill
  (Default|CallOnKill)
  (CallFunction|KillEffect)
  (Rendering|SetActorHiddenInGame true)
  (Collision|SetActorEnableCollision false)
  (Actor|SetLifeSpan 1e+01))

(event Custom|PlayEffect
  ;[1 1 1] エフェクト系
  (Effects|SpawnEmitteratLocation "/Game/PON/Particles/P_HitSpark.P_HitSpark" (Transformation|GetActorLocation))
  (Audio|PlaySound2D "/Game/PON/Sounds/Hit_Cue.Hit_Cue" 1.0 1.0 0.0 0 0))

(event Custom|KillEffect
  ;[1 1 1] エフェクト系
  (Effects|SpawnEmitteratLocation "/Game/StarterContent/Particles/P_Explosion.P_Explosion" (Transformation|GetActorLocation))
  (Audio|PlaySound2D "/Game/PON/Sounds/Bomb_Cue.Bomb_Cue" 1.0 1.0 0.0 0 0))

(event EventTick
  (params (DeltaSeconds :type Float%20%28single-precision%29))
  (CallFunction|Move))

(fn ConstructionScript)