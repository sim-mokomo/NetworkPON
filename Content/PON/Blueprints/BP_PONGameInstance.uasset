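; Game instance for PON that handles hosting and joining two-player LAN multiplayer sessions.
; OpenHost creates a session and, on success, opens the Game level as a listen server.
; JoinAsClient searches for LAN sessions and joins the first result without letting the player choose.
; Session steps print debug messages, and network and travel error handlers only print the failure type on screen, with no recovery.
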(event Custom|OpenHost
  (|Session (Game|GetPlayerController 0) 2 true
    (:OnSuccess
      (Development|PrintString "Create Session")
      (Game|OpenLevel(byName) "Game" true "listen"))))

(event Custom|JoinAsClient
  (bind _results (|FindSessions (Game|GetPlayerController 0) 2 true)
    (:OnSuccess
      (Development|PrintString "Find Session")
      (|JoinSession (Game|GetPlayerController 0) (Utilities|Array|Get(acopy) _results)
        (:OnSuccess
          (Development|PrintString "Join Sessino"))
        (:OnFailure
          (Development|PrintString "Failed to Join Sessino"))))))

(event EventHandleNetworkError
  (params (FailureType :type ENetworkFailure%20Enum :default "NetDriverAlreadyExists") (bIsServer :type Boolean))
  (switch Utilities|FlowControl|Switch|SwitchonENetworkFailure FailureType
    (:NetDriverAlreadyExists
      _)
    (:NetDriverCreateFailure
      _)
    (:NetDriverListenFailure
      _)
    (:ConnectionLost
      _)
    (:ConnectionTimeout
      _)
    (:FailureReceived
      _)
    (:OutdatedClient
      _)
    (:OutdatedServer
      _)
    (:PendingConnectionFailure
      _)
    (:NetGuidMismatch
      _)
    (:NetChecksumMismatch
      _))
  (Development|PrintString (Utilities|String|EnumtoString FailureType) true true "(R=0.000000,G=0.660000,B=1.000000,A=1.000000)" 2e+01))

(event EventHandleTravelError
  (params (FailureType :type ETravelFailure%20Enum :default "NoLevel"))
  (switch Utilities|FlowControl|Switch|SwitchonETravelFailure FailureType
    (:NoLevel
      _)
    (:LoadMapFailure
      _)
    (:InvalidURL
      _)
    (:PackageMissing
      _)
    (:PackageVersion
      _)
    (:NoDownload
      _)
    (:TravelFailure
      _)
    (:CheatCommands
      _)
    (:PendingNetGameCreateFailure
      _)
    (:CloudSaveFailure
      _)
    (:ServerTravelFailure
      _)
    (:ClientTravelFailure
      _))
  (Development|PrintString (Utilities|String|EnumtoString FailureType) true true "(R=0.000000,G=0.660000,B=1.000000,A=1.000000)" 2e+01))