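; BP_GameCtrl is a game controller for PON that sets the player's view and holds player-spawning logic.
; One second after BeginPlay, it points player controller 0 at the first BP_PONGameCamera and prints a debug message.
; CreatePlayer spawns a BP_Bar at each PlayerStart into Players, and ConnectCtrl stubs a server/client authority check.
; The calls to both events are unwired, so only the camera setup runs here.
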(event Custom|CreatePlayer
  (bind _outactors (Actor|GetAllActorsOfClass "/Script/Engine.PlayerStart"))
  (for _array_element _outactors
    (bind _returnvalue (Game|SpawnActorfromClass "/Game/PON/Blueprints/BP_Bar.BP_Bar_C" (Transformation|GetActorTransform _array_element) "Undefined" 0 0))
    (Utilities|Array|Add (Variables|Default|GetPlayers) _returnvalue)))

(event Custom|SettingPlayerCamera
  ;[1 1 1] カメラを標準位置に設定する。
  (bind _outactors (Actor|GetAllActorsOfClass "/Game/PON/Blueprints/BP_PONGameCamera.BP_PONGameCamera_C"))
  (Game|Player|SetViewTargetwithBlend (Game|GetPlayerController 0) (Utilities|Array|Get(acopy) _outactors) 0.0 "VTBlend_Linear" 0.0 false)
  (Development|PrintString "Setting Camera" true true "(R=0.000000,G=0.660000,B=1.000000,A=1.000000)" 1e+02))

(event Custom|ConnectCtrl
  (Utilities|CheckIsServerorClient)
  (Networking|SwitchHasAuthority))

(event EventBeginPlay
  (Utilities|FlowControl|Delay 1.0)
  (CallFunction|SettingPlayerCamera))

(fn ConstructionScript)