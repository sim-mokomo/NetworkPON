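; Player controller for the PON game that spawns and possesses a paddle (BP_Bar) for its player and switches to the shared game camera.
; On BeginPlay, SpawnBarOnServer uses BP_PONGame's bar count to choose name and spawn transform, then registers the bar with the game mode.
; An OnSpawnBar event triggers the delayed view-target switch.
; Authority-based helpers for PlayerStart lookup and player names are defined but unused in this graph.
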(event Custom|SettingCamera
  ;[1 1 1] カメラをゲームカメラに設定
  (bind _asbp_pongame (Utilities|Casting|CastToBP_PONGame (Game|GetGameMode)))
  (Game|Player|SetViewTargetwithBlend (Default|GetGameCamera _asbp_pongame) 0.0 "VTBlend_Linear" 0.0 false))

(event Custom|SpawnBarOnServer
  ;[1 1 1] バーを生成
  (bind _asbp_pongame (Utilities|Casting|CastToBP_PONGame (Game|GetGameMode))
    (:then
      (bind _num (Default|GetBarNum _asbp_pongame))
      (if (<= _num 1)
        (bind _spawntrans (Default|GetSpawnTrans _asbp_pongame (Utilities|String|StringToName (Utilities|String|ToString(Integer) (+ _num 1))) :!label _label))
        (bind _returnvalue (Game|SpawnActorfromClass "/Game/PON/Blueprints/BP_Bar.BP_Bar_C" _spawntrans "Undefined" 0 (Utilities|String|StringToName (Utilities|String|BuildString(Integer) "" "Player" (+ _num 1))) 0))
        (Default|AddPlayer _asbp_pongame _returnvalue)
        (Pawn|Possess _returnvalue)
        (Default|CallOnSpawnBar _returnvalue)))
    (:CastFailed
      (goto _label))))

(event Custom|OnSpawnBar_Event
  (params (SpawnBar :type BP%20Bar%20Object%20Reference))
  ;[1 1 1] 生成終了後にカメラを設定
  (Utilities|FlowControl|Delay 1.0)
  (CallFunction|SettingCamera))

(event EventBeginPlay
  ;[1 1 1] 生成終了後にカメラを設定
  (EventDispatchers|BindEventtoOnSpawnBar (delegate Custom|OnSpawnBar_Event))
  (CallFunction|SpawnBaronServer))

(fn ConstructionScript)

(fn GetSpawnTrans
  ;[1 1 1] クライアント/サーバーごとに指定の生成位置を取得
  (Networking|SwitchHasAuthority
    (:Authority
      (LocalVariables|SetTargetID "1"))
    (:Remote
      (LocalVariables|SetTargetID "2")))
  (bind _outactors (Actor|GetAllActorsOfClass "/Script/Engine.PlayerStart"))
  (for _array_element _outactors
    (if (Utilities|Name|Equal(Name) (Variables|/Script/Engine.PlayerStart|GetPlayerStartTag _array_element) (LocalVariables|GetTargetID))
      (return (Transformation|GetActorTransform _array_element)))))

(fn GetPlayerName
  (Networking|SwitchHasAuthority
    (:Authority
      (return "Player1"))
    (:Remote
      (return "Player2"))))